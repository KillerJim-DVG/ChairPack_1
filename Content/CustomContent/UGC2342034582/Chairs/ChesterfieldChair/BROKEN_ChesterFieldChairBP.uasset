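; Interactive Chesterfield chair (marked BROKEN in its name) that seats one player at a time.
; Box overlap shows a local widget and enables E to send an Interaction; end overlap waits for replication before possibly disabling input.
; Server-side PlayerInteracting toggles the seated animation and attaches the pawn at SnapPoint without movement or collision, or ejects it at EjectPoint.
; Destruction resets any seated pawn and removes the widget.
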(event `self.ReceiveDestroyed`
  ;[1 1 1] If destroyed (removed, etc.) make sure we remove anything the playe rmight be seeing
  (`/Game/CustomContent/UGC2342034582/Library/KJModMacroLibrary.HandleClientServerLogic`
    (:`ServerLogic`
      ;;[1 0.5152 0.05805] If a player is sitting on us (client or server) then we reset the pawn to enable them to move on our destruction
      (if (`KismetSystemLibrary.IsValid` (`self.SeatedPlayer`))
        (`KJModPlayerProxy.ResetPawnToDefaults` (`self.SeatedPlayer`))))
    (:`ClientLogic`
      (`/Engine/EditorBlueprintResources/StandardMacros.IsValid` (`self.Widget`)
        (:`Is Valid`
          (`Widget.RemoveFromParent` (`self.Widget`)))))))

(event `Key|E`
  (params (Key :type "Key Structure"))
  ;[1 1 1] CLIENT - Handle E press
  (:`Pressed`
    (`KJModInteractionActor.Interaction` (`GameplayStatics.GetPlayerController` 0) self true "E")))

(event `self.Box.OnComponentBeginOverlap`
  (params (OverlappedComponent :type "PrimitiveComponent Object Reference") (OtherActor :type "Actor Object Reference") (OtherComp :type "PrimitiveComponent Object Reference") (OtherBodyIndex :type Integer) (bFromSweep :type Boolean) (SweepResult :type "HitResult Structure (by ref)"))
  ;[1 1 1] BEGIN OVERLAP - Show UI and accept input
  (bind _aspawn (cast `Pawn` OtherActor))
  (if (`Pawn.IsLocallyControlled` _aspawn)
    (if (not (`self.PlayerSeated`))
      (bind _returnvalue (`|CreateWidget` "/Game/CustomContent/UGC2342034582/Chairs/ChesterfieldChair/Widget/ChesterfieldChairWidget.ChesterfieldChairWidget_C" (`GameplayStatics.GetPlayerController` 0)))
      (bind _output_get (set `self.Widget` _returnvalue))
      (`UserWidget.AddToViewport` _output_get 0)
      (`self.EnableInput` (`GameplayStatics.GetPlayerController` 0)))))

(event `self.Box.OnComponentEndOverlap`
  (params (OverlappedComponent :type "PrimitiveComponent Object Reference") (OtherActor :type "Actor Object Reference") (OtherComp :type "PrimitiveComponent Object Reference") (OtherBodyIndex :type Integer))
  ;[1 1 1] END OVERLAP - Occurs when player leaves box overlap OR (and critically) when the pawn is set to no collide - Remove UI and disable input#
  (bind _aspawn (cast `Pawn` OtherActor))
  (if (`Pawn.IsLocallyControlled` _aspawn)
    (`/Engine/EditorBlueprintResources/StandardMacros.IsValid` (`self.Widget`)
      (:`Is Valid`
        (`Widget.RemoveFromParent` (`self.Widget`))
        (`KismetSystemLibrary.Delay` 0.5) ; Wait for PlayerSeated and SeatedPlayer to be replicated out from server to us locally..
        (if (not (or (not (`self.PlayerSeated`)) (== (`self.SeatedPlayer`) (`GameplayStatics.GetPlayerController` 0))))
          (`self.DisableInput` (`GameplayStatics.GetPlayerController` 0)))))))

(event `KJModInteractableObjectInterface.PlayerInteracting`
  (params (interactingPlayerProxy :type "KJModPlayerProxy Object Reference") (playerController :type "PlayerController Object Reference") (active :type Boolean) (inputChord :type "InputChord Structure") (cookie :type Integer))
  ;[1 1 1] SERVER INTERACTION - SPACE pressed on a client
  ;;[1 1 1] Ensure onnly one person can sit down at a time, and that this person can get up
  (`/Engine/EditorBlueprintResources/StandardMacros.IsValid` (`self.SeatedPlayer`)
    (:`Is Valid`
      (if (`self.PlayerSeated`)
        (if (== playerController (`self.SeatedPlayer`))
          (bind _output_get (set `self.PlayerSeated` (not (`self.PlayerSeated`)) :!label _label))
          (`KJModPlayerProxy.OverrideAnimations` playerController (select `bool` _output_get :`false` "NoOverride" :`true` "SeatedIdle" :!type "EKJModAnimationOverride Enum"))
          (`self.WeldPlayerServer` (`Controller.K2_GetPawn` playerController) _output_get)
          (if _output_get
            (set `self.SeatedPlayer` playerController)
            (else
              (set `self.SeatedPlayer` null))))
        (else
          (goto _label))))
    (:`Is Not Valid`
      (goto _label))))

(event `WeldPlayerServer`
  (params (PlayerToWeld :type "Pawn Object Reference") (RequiresSeating :type Boolean))
  (bind _returnvalue (`self.GetComponentByClass` PlayerToWeld "/Script/Engine.SkeletalMeshComponent"))
  (bind _returnvalue_2 (`self.GetComponentByClass` PlayerToWeld "/Script/Engine.CapsuleComponent"))
  (bind _returnvalue_3 (`self.GetComponentByClass` PlayerToWeld "/Script/Engine.CapsuleComponent"))
  (bind _returnvalue_4 (`self.GetComponentByClass` PlayerToWeld "/Script/Engine.SkeletalMeshComponent"))
  (bind _snappoint (`self.SnapPoint`))
  (bind _ejectpoint (`self.EjectPoint`))
  ;[1 1 1] WELD PLAYER - Sit player down
  (if RequiresSeating
    (bind _ascharacter_movement_component (cast `CharacterMovementComponent` (`Pawn.GetMovementComponent` PlayerToWeld)))
    (`CharacterMovementComponent.SetMovementMode` _ascharacter_movement_component "MOVE_None" 0)
    (set `Pawn.bUseControllerRotationYaw` false PlayerToWeld)
    (`self.K2_SetActorLocationAndRotation` PlayerToWeld (`SceneComponent.K2_GetComponentLocation` _snappoint) (`SceneComponent.K2_GetComponentRotation` _snappoint) false true)
    (`self.K2_AttachToActor` PlayerToWeld self "None" "KeepWorld" "KeepWorld" "KeepWorld" true)
    (`|ExecutionSequence`
      (:`then_0`
        (`PrimitiveComponent.SetCollisionProfileName` _returnvalue_3 "None" true)
        (`PrimitiveComponent.SetCollisionEnabled` _returnvalue_3 "NoCollision"))
      (:`then_1`
        (`PrimitiveComponent.SetCollisionProfileName` _returnvalue_4 "None" true)
        (`PrimitiveComponent.SetCollisionEnabled` _returnvalue_4 "NoCollision")))
    (else
      (bind _ascharacter_movement_component_2 (cast `CharacterMovementComponent` (`Pawn.GetMovementComponent` PlayerToWeld)))
      (`CharacterMovementComponent.SetMovementMode` _ascharacter_movement_component_2 "MOVE_Walking" 0)
      (set `Pawn.bUseControllerRotationYaw` true PlayerToWeld)
      (`self.K2_SetActorLocationAndRotation` PlayerToWeld (`SceneComponent.K2_GetComponentLocation` _ejectpoint) (`SceneComponent.K2_GetComponentRotation` _ejectpoint) false true)
      (`self.K2_DetachFromActor` PlayerToWeld "KeepWorld" "KeepWorld" "KeepWorld")
      (`|ExecutionSequence`
        (:`then_0`
          (`PrimitiveComponent.SetCollisionProfileName` _returnvalue_2 "Pawn" true)
          (`PrimitiveComponent.SetCollisionEnabled` _returnvalue_2 "QueryAndPhysics"))
        (:`then_1`
          (`PrimitiveComponent.SetCollisionProfileName` _returnvalue "Pawn" true)
          (`PrimitiveComponent.SetCollisionEnabled` _returnvalue "QueryAndPhysics"))))))

(fn `UserConstructionScript`)