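; Base multiplayer chair that lets one player at a time sit down and get up.
; Box overlap shows a local prompt widget and enables E input, which triggers server-side seat toggling.
; Sitting overrides animation, snaps and attaches the pawn, and disables movement and collision; standing reverses this at an eject point.
; Replicated seat state keeps input enabled for the sitter after a delayed check and restores the pawn if the chair is destroyed.
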(event `self.ReceiveDestroyed`
  (bind _seatedpawn (`self.SeatedPawn`))
  (bind _returnvalue (`self.GetComponentByClass` _seatedpawn "/Script/Engine.SkeletalMeshComponent"))
  (bind _returnvalue_2 (`self.GetComponentByClass` _seatedpawn "/Script/Engine.CapsuleComponent"))
  ;[1 1 1] If destroyed (removed, etc.) make sure we remove anything the playe rmight be seeing
  (`/Game/CustomContent/UGC2342034582/Library/KJModMacroLibrary.HandleClientServerLogic`
    (:`ServerLogic`
      _)
    (:`ClientLogic`
      ;;[1 1 1] Clients? Get rid of UI if it's there
      (if (`self.ShowingUILocally`)
        (`Widget.RemoveFromParent` (`self.Widget`)))))
  ;;[1 0.5152 0.05805] If a player is sitting on us (client or server) and the chair was destroyed, then we need to reset the pawn so we see them (i.e .the server or client) standing correctly (otherwise they has no collision, fall through things, look like they're flying, etc.)
  (if (`KismetSystemLibrary.IsValid` (`self.SeatedPawn`))
    (`KJModPlayerProxy.ResetPawnToDefaults` (`self.SeatedPlayer`))
    (bind _ascharacter_movement_component (cast `CharacterMovementComponent` (`Pawn.GetMovementComponent` _seatedpawn)))
    (`CharacterMovementComponent.SetMovementMode` _ascharacter_movement_component "MOVE_Walking" 0)
    (set `Pawn.bUseControllerRotationYaw` true _seatedpawn)
    (`|ExecutionSequence`
      (:`then_0`
        (`PrimitiveComponent.SetCollisionProfileName` _returnvalue_2 "Pawn" true)
        (`PrimitiveComponent.SetCollisionEnabled` _returnvalue_2 "QueryAndPhysics"))
      (:`then_1`
        (`PrimitiveComponent.SetCollisionProfileName` _returnvalue "Pawn" true)
        (`PrimitiveComponent.SetCollisionEnabled` _returnvalue "QueryAndPhysics")))))

(event `Key|E`
  (params (Key :type "Key Structure"))
  ;[1 1 1] CLIENT - Handle E press
  (:`Pressed`
    (`KJModInteractionActor.Interaction` (`GameplayStatics.GetPlayerController` 0) self true "E")))

(event `self.Box.OnComponentBeginOverlap`
  (params (OverlappedComponent :type "PrimitiveComponent Object Reference") (OtherActor :type "Actor Object Reference") (OtherComp :type "PrimitiveComponent Object Reference") (OtherBodyIndex :type Integer) (bFromSweep :type Boolean) (SweepResult :type "HitResult Structure (by ref)"))
  ;[1 1 1] BEGIN OVERLAP - Show UI and accept input
  (bind _aspawn (cast `Pawn` OtherActor))
  (if (`Pawn.IsLocallyControlled` _aspawn)
    (if (`self.PlayerSeated`)
      _
      (elif (not (`self.ShowingUILocally`))
        (bind _returnvalue (`|CreateWidget` "/Game/CustomContent/UGC2342034582/Chairs/ChesterfieldChair/Widget/ChesterfieldChairWidget.ChesterfieldChairWidget_C" (`GameplayStatics.GetPlayerController` 0)))
        (bind _output_get (set `self.Widget` _returnvalue))
        (`UserWidget.AddToViewport` _output_get 0)
        (set `self.ShowingUILocally` true)
        (`self.EnableInput` (`GameplayStatics.GetPlayerController` 0))))))

(event `self.Box.OnComponentEndOverlap`
  (params (OverlappedComponent :type "PrimitiveComponent Object Reference") (OtherActor :type "Actor Object Reference") (OtherComp :type "PrimitiveComponent Object Reference") (OtherBodyIndex :type Integer))
  ;[1 1 1] END OVERLAP - Occurs when player leaves box overlap OR (and critically) when the pawn is set to no collide - Remove UI and disable input#
  (bind _aspawn (cast `Pawn` OtherActor))
  (if (`Pawn.IsLocallyControlled` _aspawn)
    (if (`self.ShowingUILocally`)
      (`Widget.RemoveFromParent` (`self.Widget`))
      (set `self.Widget` null)
      (set `self.ShowingUILocally` false))
    (`KismetSystemLibrary.Delay` 0.5) ; Wait for PlayerSeated and SeatedPlayer to be replicated out from server to us locally..
    (if (or (not (`self.PlayerSeated`)) (not (== (`self.SeatedPlayer`) (`GameplayStatics.GetPlayerController` 0))))
      (`self.DisableInput` (`GameplayStatics.GetPlayerController` 0))
      (`KismetSystemLibrary.PrintString` "Disabled input")
      (else
        (`KismetSystemLibrary.PrintString` "Dit not Disable input")))))

(event `KJModInteractableObjectInterface.PlayerInteracting`
  (params (interactingPlayerProxy :type "KJModPlayerProxy Object Reference") (playerController :type "PlayerController Object Reference") (active :type Boolean) (inputChord :type "InputChord Structure") (cookie :type Integer))
  ;[1 1 1] SERVER INTERACTION - SPACE pressed on a client
  ;;[1 1 1] Ensure only one person can sit down at a time, and that this person can get up
  (`/Engine/EditorBlueprintResources/StandardMacros.IsValid` (`self.SeatedPlayer`)
    (:`Is Valid`
      (if (`self.PlayerSeated`)
        (if (== playerController (`self.SeatedPlayer`))
          (bind _output_get (set `self.PlayerSeated` (not (`self.PlayerSeated`)) :!label _label))
          (`KJModPlayerProxy.OverrideAnimations` playerController (select `bool` _output_get :`false` "NoOverride" :`true` "SeatedIdle" :!type "EKJModAnimationOverride Enum"))
          (`self.WeldPlayerServer` (`Controller.K2_GetPawn` playerController) _output_get)
          (if _output_get
            (bind _output_get_2 (set `self.SeatedPlayer` playerController))
            ;;[1 0.8201 0.05535] Replicate this, so that if the chair is destroyed we can "fix" the sitting player on remote clients (i.e. make them stand, no fall through stuff, etc.) - this was added late in the design; we would have ideally just had one replicated variable but this was a quick fix
            (set `self.SeatedPawn` (`Controller.K2_GetPawn` _output_get_2))
            (else
              (`KJModPlayerProxy.ResetPawnToDefaults` playerController)
              (set `self.SeatedPlayer` null)
              (set `self.SeatedPawn` null))))
        (else
          (goto _label))))
    (:`Is Not Valid`
      (goto _label))))

(event `WeldPlayerServer`
  (params (PlayerToWeld :type "Pawn Object Reference") (RequiresSeating :type Boolean))
  (bind _returnvalue (`self.GetComponentByClass` PlayerToWeld "/Script/Engine.CapsuleComponent"))
  (bind _returnvalue_2 (`self.GetComponentByClass` PlayerToWeld "/Script/Engine.SkeletalMeshComponent"))
  (bind _returnvalue_3 (`self.GetComponentByClass` PlayerToWeld "/Script/Engine.CapsuleComponent"))
  (bind _returnvalue_4 (`self.GetComponentByClass` PlayerToWeld "/Script/Engine.SkeletalMeshComponent"))
  (bind _snappoint (`self.SnapPoint`))
  (bind _ejectpoint (`self.EjectPoint`))
  ;[1 1 1] WELD PLAYER - Sit player down. We set our animation to be overriden to "seated", we attach the player so they stick to the chair and then disable collision so the chair + pawn don't fight and cause you to fly off (or we inverse this for getting up)
  (if RequiresSeating
    (bind _ascharacter_movement_component (cast `CharacterMovementComponent` (`Pawn.GetMovementComponent` PlayerToWeld)))
    (`CharacterMovementComponent.SetMovementMode` _ascharacter_movement_component "MOVE_None" 0)
    (set `Pawn.bUseControllerRotationYaw` false PlayerToWeld)
    (`self.K2_SetActorLocationAndRotation` PlayerToWeld (`SceneComponent.K2_GetComponentLocation` _snappoint) (`SceneComponent.K2_GetComponentRotation` _snappoint) false true)
    (`self.K2_AttachToActor` PlayerToWeld self "None" "KeepWorld" "KeepWorld" "KeepWorld" true)
    (`|ExecutionSequence`
      (:`then_0`
        (`PrimitiveComponent.SetCollisionProfileName` _returnvalue "None" true)
        (`PrimitiveComponent.SetCollisionEnabled` _returnvalue "NoCollision"))
      (:`then_1`
        (`PrimitiveComponent.SetCollisionProfileName` _returnvalue_2 "None" true)
        (`PrimitiveComponent.SetCollisionEnabled` _returnvalue_2 "NoCollision")))
    (else
      (bind _ascharacter_movement_component_2 (cast `CharacterMovementComponent` (`Pawn.GetMovementComponent` PlayerToWeld)))
      (`CharacterMovementComponent.SetMovementMode` _ascharacter_movement_component_2 "MOVE_Walking" 0)
      (set `Pawn.bUseControllerRotationYaw` true PlayerToWeld)
      (`self.K2_SetActorLocationAndRotation` PlayerToWeld (`SceneComponent.K2_GetComponentLocation` _ejectpoint) (`SceneComponent.K2_GetComponentRotation` _ejectpoint) false true)
      (`self.K2_DetachFromActor` PlayerToWeld "KeepWorld" "KeepWorld" "KeepWorld")
      (`|ExecutionSequence`
        (:`then_0`
          (`PrimitiveComponent.SetCollisionProfileName` _returnvalue_3 "Pawn" true)
          (`PrimitiveComponent.SetCollisionEnabled` _returnvalue_3 "QueryAndPhysics"))
        (:`then_1`
          (`PrimitiveComponent.SetCollisionProfileName` _returnvalue_4 "Pawn" true)
          (`PrimitiveComponent.SetCollisionEnabled` _returnvalue_4 "QueryAndPhysics"))))))

(fn `UserConstructionScript`)